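; Tunnel segment for an endless runner, with a spinning holed wall and optional banana pickup and bat hazard.
; InitStuff randomizes the wall mesh and roll, then offsets or removes each item.
; The trigger adds score and capped speed, has TunnelSpawner spawn another tunnel, then destroys this one.
; Walls and bats hit the player, bananas heal; projectiles die on all three, destroying items and scoring for bats.
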(event OnComponentBeginOverlap(TriggerZone)
  (params (OverlappedComponent :type Primitive%20Component%20Object%20Reference) (OtherActor :type Actor%20Object%20Reference) (OtherComp :type Primitive%20Component%20Object%20Reference) (OtherBodyIndex :type Integer) (bFromSweep :type Boolean) (SweepResult :type Hit%20Result%20Structure%20%28by%20ref%29))
  (bind _asbp_player (Utilities|Casting|CastToBP_Player OtherActor))
  (Variables|/Game/InfiniteMatrix/Blueprints/BP_Player.BP_Player_C|SetScore _asbp_player (+ (Variables|/Game/InfiniteMatrix/Blueprints/BP_Player.BP_Player_C|GetScore _asbp_player) 1))
  (Variables|/Game/InfiniteMatrix/Blueprints/BP_Player.BP_Player_C|SetForwardSpeed _asbp_player (Math|Float|Clamp(Float) (+ (Variables|/Game/InfiniteMatrix/Blueprints/BP_Player.BP_Player_C|GetForwardSpeed _asbp_player) 2e+02) 0.0 3e+03))
  (Default|SpawnTunnelatSpawnPoint (Variables|Default|GetTunnelSpawner))
  (Actor|DestroyActor))

(event OnComponentBeginOverlap(Banana)
  (params (OverlappedComponent :type Primitive%20Component%20Object%20Reference) (OtherActor :type Actor%20Object%20Reference) (OtherComp :type Primitive%20Component%20Object%20Reference) (OtherBodyIndex :type Integer) (bFromSweep :type Boolean) (SweepResult :type Hit%20Result%20Structure%20%28by%20ref%29))
  (bind _asbp_player (Utilities|Casting|CastToBP_Player OtherActor)
    (:then
      (if (> (+ (Variables|/Game/InfiniteMatrix/Blueprints/BP_Player.BP_Player_C|GetHealth _asbp_player) 0.2) 1.1)
        _
        (else
          (Variables|/Game/InfiniteMatrix/Blueprints/BP_Player.BP_Player_C|SetHealth _asbp_player (+ (Variables|/Game/InfiniteMatrix/Blueprints/BP_Player.BP_Player_C|GetHealth _asbp_player) 0.2))))
      (Components|DestroyComponent (Variables|Default|GetBanana)))
    (:CastFailed
      (bind _asbp_projectile (Utilities|Casting|CastToBP_Projectile OtherActor))
      (Components|DestroyComponent (Variables|Default|GetBanana))
      (Actor|DestroyActor _asbp_projectile))))

(event OnComponentBeginOverlap(WallMesh)
  (params (OverlappedComponent :type Primitive%20Component%20Object%20Reference) (OtherActor :type Actor%20Object%20Reference) (OtherComp :type Primitive%20Component%20Object%20Reference) (OtherBodyIndex :type Integer) (bFromSweep :type Boolean) (SweepResult :type Hit%20Result%20Structure%20%28by%20ref%29))
  (bind _asbp_player (Utilities|Casting|CastToBP_Player OtherActor)
    (:then
      (Default|ProcessHit _asbp_player))
    (:CastFailed
      (bind _asbp_projectile (Utilities|Casting|CastToBP_Projectile OtherActor))
      (Actor|DestroyActor _asbp_projectile))))

(event OnComponentBeginOverlap(Bat)
  (params (OverlappedComponent :type Primitive%20Component%20Object%20Reference) (OtherActor :type Actor%20Object%20Reference) (OtherComp :type Primitive%20Component%20Object%20Reference) (OtherBodyIndex :type Integer) (bFromSweep :type Boolean) (SweepResult :type Hit%20Result%20Structure%20%28by%20ref%29))
  (bind _asbp_player (Utilities|Casting|CastToBP_Player OtherActor)
    (:then
      (Default|ProcessHit _asbp_player)
      (Components|DestroyComponent (Variables|Default|GetBat)))
    (:CastFailed
      (bind _asbp_projectile (Utilities|Casting|CastToBP_Projectile OtherActor))
      (Components|DestroyComponent (Variables|Default|GetBat))
      (Actor|DestroyActor _asbp_projectile)
      (bind _outactors (Actor|GetAllActorsOfClass "/Game/InfiniteMatrix/Blueprints/BP_Player.BP_Player_C"))
      (for _array_element _outactors
        (Variables|/Game/InfiniteMatrix/Blueprints/BP_Player.BP_Player_C|SetScore _array_element (+ (Variables|/Game/InfiniteMatrix/Blueprints/BP_Player.BP_Player_C|GetScore _array_element) 1))))))

(event EventBeginPlay)

(event EventTick
  (params (DeltaSeconds :type Float%20%28single-precision%29))
  (Transformation|AddLocalRotation (Variables|Default|GetWallMesh) (Math|Rotator|MakeRotator (* DeltaSeconds (Variables|Default|GetRotateSpeed)) 0.0 0.0) false false)
  (Utilities|IsValid (Variables|Default|GetBanana)
    (:Is%20Valid
      (Transformation|AddLocalRotation (Variables|Default|GetBanana) (Math|Rotator|MakeRotator 0.0 0.0 (* DeltaSeconds (Variables|Default|GetBananaRotate))) false false)
      (Utilities|IsValid (Variables|Default|GetBat)
        (:Is%20Valid
          (Transformation|AddLocalRotation (Variables|Default|GetBat) (Math|Rotator|MakeRotator 0.0 0.0 (* (Variables|Default|GetBananaRotate) DeltaSeconds)) false false))))))

(fn ConstructionScript)

(fn RandomizeWall
  (Components|StaticMesh|SetStaticMesh (Variables|Default|GetWallMesh) (Utilities|Select :Index (Math|Random|RandomIntegerinRange 0 3) :Option%200 "/Game/InfiniteMatrix/Meshes/SM_Hole_01.SM_Hole_01" :Option%201 "/Game/InfiniteMatrix/Meshes/SM_Hole_02.SM_Hole_02" :Option%202 "/Game/InfiniteMatrix/Meshes/SM_Hole_03.SM_Hole_03" :Option%203 "/Game/InfiniteMatrix/Meshes/SM_Hole_04.SM_Hole_04"))
  (Transformation|AddLocalRotation (Variables|Default|GetWallMesh) (Math|Rotator|MakeRotator (Math|Random|RandomFloatinRange 0.0 3.6e+02) 0.0 0.0) false false))

(fn RandomizeBanana
  (Utilities|IsValid (Variables|Default|GetBanana)
    (:Is%20Valid
      (if (> (Math|Random|RandomFloatinRange 0.0 1.0) 0.8)
        (Transformation|AddLocalOffset (Variables|Default|GetBanana) (Math|Vector|MakeVector (Math|Random|RandomFloatinRange 1e+03 1.5e+03) (Math|Random|RandomFloatinRange -1.5e+02 1.5e+02) (Math|Random|RandomFloatinRange -1.5e+02 1.5e+02)) false false)
        (else
          (Components|DestroyComponent (Variables|Default|GetBanana)))))))

(fn RandomizeBat
  (Utilities|IsValid (Variables|Default|GetBat)
    (:Is%20Valid
      (if (> (Math|Random|RandomFloatinRange 0.0 1.0) 0.8)
        (Transformation|AddLocalOffset (Variables|Default|GetBat) (Math|Vector|MakeVector (Math|Random|RandomFloatinRange -1.5e+02 1.5e+02) (Math|Random|RandomFloatinRange 1e+03 1.5e+03) (Math|Random|RandomFloatinRange -1.5e+02 1.5e+02)) false false)
        (else
          (Components|DestroyComponent (Variables|Default|GetBat)))))))

(fn InitStuff
  (CallFunction|RandomizeWall)
  (CallFunction|RandomizeBanana)
  (CallFunction|RandomizeBat))